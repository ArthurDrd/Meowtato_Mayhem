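; Game mode for a local multiplayer match that ends on a time limit or a last player standing check.
; BeginPlay shows a timed intro widget, adds HUD and timer widgets, then creates a player and possessed character with its own mesh per PlayerStart.
; A looping timer updates the clock and, at the limit, destroys characters below the best score.
; A sole survivor's mesh is stored in the game instance before loading the winner level.
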(event Custom|CheckWinner
  ;[0.333 0.5702 1] Winner
  (bind _outactors (Actor|GetAllActorsOfClass "/Game/Game/Blueprints/Character/BP_Character.BP_Character_C"))
  (if (== (Utilities|Array|Length _outactors) 1)
    (bind _asbp_game_instance (Utilities|Casting|CastToBP_GameInstance (Game|GetGameInstance)))
    (Variables|/Game/Game/Blueprints/GameInstance/BP_GameInstance.BP_GameInstance_C|SetWinnerMesh _asbp_game_instance (Components|SkeletalMesh|GetSkeletalMeshAsset (Variables|/Script/Engine.Character|GetMesh (Utilities|Array|Get(acopy) _outactors))))
    (Game|OpenLevel(byName) "LVL_Winner")))

(event Custom|CallTime
  ;[0 1 0.006928] Timer
  (bind _output_get (Variables|Default|SetTime (+ (Variables|Default|GetTime) 1.0)))
  (Default|UpdateTimer (Variables|Default|GetHudTimer) _output_get)
  (if (>= (Variables|Default|GetTime) 3e+02)
    (CallFunction|CheckWinnerbyTime)
    (Utilities|Time|ClearandInvalidateTimerbyHandle (Variables|Default|GetTimer))))

(event Custom|CheckWinnerByTime
  ;[1 0 0.4044] Check Winner after the timer
  (bind _outactors (Actor|GetAllActorsOfClass "/Game/Game/Blueprints/Character/BP_Character.BP_Character_C"))
  (for _array_element _outactors
    (if (> (Variables|/Game/Game/Blueprints/Character/BP_Character.BP_Character_C|GetScore _array_element) (Variables|Default|GetBestScore))
      (Variables|Default|SetBestScore (Variables|/Game/Game/Blueprints/Character/BP_Character.BP_Character_C|GetScore _array_element))
      (Variables|Default|SetBestPlayer _array_element)))
  (for _array_element_2 _outactors
    (if (< (Variables|/Game/Game/Blueprints/Character/BP_Character.BP_Character_C|GetScore _array_element_2) (Variables|Default|GetBestScore))
      (Actor|DestroyActor _array_element_2)))
  (CallFunction|CheckWinner))

(event EventBeginPlay
  (bind _returnvalue (Game|GetPlayerController 0))
  ;[1 0.3514 0.6742] Local Multiplayer System
  (Audio|PlaySound2D "/Game/Game/Songs/Themes/keys-of-moon-immense_chosic_com_.keys-of-moon-immense_chosic_com_" 0.2 1.0 0.0 0 0)
  (Input|SetInputModeGameOnly _returnvalue false)
  (Variables|/Script/Engine.PlayerController|SetbShowMouseCursor _returnvalue false)
  (bind _returnvalue_2 (UserInterface|CreateWidget "/Game/Game/Blueprints/UI/WBP_PNJ.WBP_PNJ_C"))
  (bind _output_get (Variables|Default|SetHudPNJ _returnvalue_2))
  (UserInterface|Viewport|AddtoViewport _output_get 0)
  (Utilities|FlowControl|Delay 1e+01)
  (Widget|RemovefromParent (Variables|Default|GetHudPNJ))
  (bind _returnvalue_3 (UserInterface|CreateWidget "/Game/Game/Blueprints/UI/WBP_Hud.WBP_Hud_C"))
  (bind _output_get_2 (Variables|Default|SetHud _returnvalue_3))
  (UserInterface|Viewport|AddtoViewport _output_get_2 0)
  (bind _returnvalue_4 (UserInterface|CreateWidget "/Game/Game/Blueprints/UI/WBP_Timer.WBP_Timer_C"))
  (bind _output_get_3 (Variables|Default|SetHudTimer _returnvalue_4))
  (UserInterface|Viewport|AddtoViewport _output_get_3 0)
  (bind _outactors (Actor|GetAllActorsOfClass "/Script/Engine.PlayerStart"))
  (for (_array_element _array_index) _outactors
    (if (>= _array_index 1)
      (Class|GameplayStatics|CreatePlayer _array_index))
    (bind _returnvalue_5 (Game|SpawnActorfromClass "/Game/Game/Blueprints/Character/BP_Character.BP_Character_C" (Transformation|GetActorTransform _array_element) "Undefined" "OverrideRootScale" 0 0))
    (Pawn|Possess (Game|GetPlayerController _array_index) _returnvalue_5)
    (Components|SkeletalMesh|SetSkeletalMeshAsset (Variables|/Script/Engine.Character|GetMesh _returnvalue_5) (Utilities|Array|Get(acopy) (Variables|Default|GetArrayMesh) _array_index))
    (bind _returnvalue_6 (Utilities|Time|SetTimerbyEvent (delegate Custom|CallTime) 1.0 true))
    (Variables|Default|SetTimer _returnvalue_6)))

(fn ConstructionScript)